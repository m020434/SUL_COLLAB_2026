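; BP_ScoreTarget is a hittable target that reports accuracy-based bonuses and bursts into confetti when hit.
; OnTargetHit runs two Sequence branches, Score and Mult, each calling CalculateAccuracyBonus with HitAccuracy and only printing the result.
; Both branches converge on DestroyActor and a Niagara confetti spawn at the actor's location, so that shared tail is wired to run twice per hit.
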(event EventOnTargetHit
  (params (HitAccuracy :type Float%20%28single-precision%29))
  (Variables|Default|SetHit%20Accuracy HitAccuracy)
  (Utilities|FlowControl|Sequence
    (:then_0
      (bind _returnvalue (CallFunction|CalculateAccuracyBonus 0 (Variables|Default|GetHit%20Accuracy))) ; For Score
      (Development|PrintString (Utilities|String|ToString(Text) (Utilities|Text|FormatText "Score Added: {scoreAdded}" _returnvalue))))
    (:then_1
      (bind _returnvalue_2 (CallFunction|CalculateAccuracyBonus 0 (Variables|Default|GetHit%20Accuracy))) ; For Mult
      (Development|PrintString (Utilities|String|ToString(Text) (Utilities|Text|FormatText "Mult Added: {multAdded}" _returnvalue_2)))))
  (Actor|DestroyActor)
  (Niagara|SpawnSystematLocation "/Game/Juno/VFX/N_Confetti_OutwardBurst.N_Confetti_OutwardBurst" (Transformation|GetActorLocation)))

(fn ConstructionScript)