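; Player character Blueprint that sets up the HUD and a temporary gun attached to the camera on BeginPlay.
; Slide start and end events play and reverse a timeline that scales capsule half-height from its default.
; Wildcard blind and damage-mitigation events are forwarded to the HUD widget, while unmitigated damage only prints a message.
; Debug keys apply self-damage and activate an example wildcard ability.
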(event Custom|OnSlideStart_Event
  ;[0.15 0.15 0.15 0.5] Slide Transition
  (bind _slide (Timeline|Timeline Play)
    (:Update
      (Components|Capsule|SetCapsuleHalfHeight (Variables|Default|GetCapsuleComponent) (* _slide (Variables|Default|GetDefault%20Height)) true))))

(event Custom|OnSlideEnd_Event
  ;[0.15 0.15 0.15 0.5] Slide Transition
  (bind _slide (Timeline|Timeline Reverse)
    (:Update
      (Components|Capsule|SetCapsuleHalfHeight (Variables|Default|GetCapsuleComponent) (* _slide (Variables|Default|GetDefault%20Height)) true))))

(event Custom|WildcardBlinds
  (Default|CallWildcard;BlindStart (Variables|Default|GetPlayerWidget)))

(event Custom|Add;Mult)

(event Game|Damage|EventAnyDamage
  (params (Damage :type Float%20%28single-precision%29) (DamageType :type Damage%20Type%20Object%20Reference) (InstigatedBy :type Controller%20Object%20Reference) (DamageCauser :type Actor%20Object%20Reference))
  ;[0.15 0.15 0.15 0.5] WC-IronSkin uses this bool for its effect, event dispatcher leads to WBP_PlayerHealth
  (if (Variables|Default|GetMitigationActive?)
    (Default|CallWildcard;MitigateStart (Variables|Default|GetPlayerWidget))
    (else
      (Development|PrintString "Take Damage"))))

(event EventBeginPlay
  (bind _gunpos (Variables|Default|GetGunPos))
  (EventDispatchers|BindEventtoWildcard;Blind (EventDispatchers|CreateEvent :!event Custom|WildcardBlinds))
  (bind _returnvalue (UserInterface|CreateWidget "/Game/Blueprint/Shez/UI/Player/WBP_PlayerHUDCORE.WBP_PlayerHUDCORE_C"))
  (bind _output_get (Variables|Default|SetPlayerWidget _returnvalue))
  (UserInterface|Viewport|AddtoViewport _output_get 0)
  (Utilities|FlowControl|Sequence
    (:then_0
      ;[0.15 0.15 0.15 0.5] Temp
      (bind _returnvalue_2 (Game|SpawnActorfromClass "/Game/Blueprint/DefaultBlueprint/BP_Gun.BP_Gun_C" (Math|Transform|MakeTransform (Variables|/Script/Engine.SceneComponent|GetRelativeLocation _gunpos) (Variables|/Script/Engine.SceneComponent|GetRelativeRotation _gunpos) "1.000000,1.000000,1.000000") "Undefined" "MultiplyWithRoot" 0 0))
      (bind _output_get_2 (Variables|Default|SetGun _returnvalue_2))
      (Transformation|AttachComponentToComponent _output_get_2 (Variables|Default|GetCamComp) "None" "KeepRelative" "KeepRelative" "KeepRelative" true))
    (:then_1
      (Variables|Default|SetDefault%20Height (Components|Capsule|GetUnscaledCapsuleHalfHeight (Variables|Default|GetCapsuleComponent))))
    (:then_2
      (EventDispatchers|BindEventtoOnSlideStart (delegate Custom|OnSlideStart_Event))
      (EventDispatchers|AssignOnSlideEnd (delegate Custom|OnSlideEnd_Event)))))

(event Input|KeyboardEvents|DebugKeyR
  (params (Key :type Key%20Structure :default "None") (ActionValue :type Input%20Action%20Value%20Structure))
  ;[0.15 0.15 0.15 0.5] Debug Activate Ability
  (:Pressed
    (Class|BaseWildcard|ActivateWildcard (Utilities|ResolveSoftReference (Variables|Default|GetAs%20BP%20Wildcard%20Example)))))

(event Input|KeyboardEvents|DebugKeyC
  (params (Key :type Key%20Structure :default "None") (ActionValue :type Input%20Action%20Value%20Structure))
  ;[0.15 0.15 0.15 0.5] Debug take damage
  (:Pressed
    (Game|Damage|ApplyDamage self 1e+01 0 0)))

(fn ConstructionScript)