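; BP_WCGambit is a gambling wildcard that registers itself with the Shez player character when its sphere is overlapped.
; On activation it makes an even-odds roll (despite a "1/6?" comment), playing a sound, then an outcome sound after that clip's duration.
; A loss blinds the player, while a win only plays audio.
; The end event is empty, and disconnected nodes hold unused mitigation and timer logic.
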(event OnComponentBeginOverlap(Sphere)
  (params (OverlappedComponent :type Primitive%20Component%20Object%20Reference) (OtherActor :type Actor%20Object%20Reference) (OtherComp :type Primitive%20Component%20Object%20Reference) (OtherBodyIndex :type Integer) (bFromSweep :type Boolean) (SweepResult :type Hit%20Result%20Structure%20%28by%20ref%29))
  (Variables|/Game/Blueprint/Shez/Class/BP_ShezPlayerCharacter.BP_ShezPlayerCharacter_C|SetAs%20BP%20Wildcard%20Example (Variables|Default|GetPlayerCharacterRef) (Utilities|ResolveSoftReference self)))

(event EventBeginPlay
  (bind _asbp_shez_player_character (Utilities|Casting|CastToBP_ShezPlayerCharacter (Game|Player|GetPlayerPawn 0)))
  (Variables|Default|SetPlayerCharacterRef _asbp_shez_player_character))

(event EventOnWildcardEnd)

(event EventOnWildcardActivate
  (bind _sound (Variables|Default|GetSound))
  (bind _sound_0 (Variables|Default|GetSound_0))
  (if (>= (Math|Random|RandomIntegerinRange 0 5) 3)
    ;[0.15 0.15 0.15 0.5] Loss
    (Audio|PlaySound2D _sound 1.0 1.0 0.0 0 0)
    (Utilities|FlowControl|Delay (Variables|/Script/Engine.SoundBase|GetDuration _sound))
    (Audio|PlaySound2D "/Game/Blueprint/Shez/SFX_WC_RouletteLoss1.SFX_WC_RouletteLoss1" 1.0 1.0 0.0 0 0)
    (Default|CallWildcard;Blind (Variables|Default|GetPlayerCharacterRef))
    (else
      ;[0.15 0.15 0.15 0.5] Win
      (Audio|PlaySound2D _sound_0 1.0 1.0 0.0 0 0)
      (Utilities|FlowControl|Delay (Variables|/Script/Engine.SoundBase|GetDuration _sound_0))
      (Audio|PlaySound2D "/Game/Blueprint/Shez/floraphonic-playful-casino-slot-machine-bonus-1-183918.floraphonic-playful-casino-slot-machine-bonus-1-183918" 1.0 1.0 0.0 0 0))))

(fn ConstructionScript)