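; Wildcard ability "The World" that stops time around the player, with Za Warudo sound effects.
; On activation it applies a color grade to the player camera, starts the wildcard timer, drops global time dilation to near zero and raises the player's custom dilation to compensate.
; On end it plays the resume sound, waits a dilation-scaled delay, resets the grade, restores both dilations and reports the wildcard finished.
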(event OnComponentBeginOverlap(Sphere)
  (params (OverlappedComponent :type Primitive%20Component%20Object%20Reference) (OtherActor :type Actor%20Object%20Reference) (OtherComp :type Primitive%20Component%20Object%20Reference) (OtherBodyIndex :type Integer) (bFromSweep :type Boolean) (SweepResult :type Hit%20Result%20Structure%20%28by%20ref%29)))

(event EventBeginPlay
  (bind _asbp_default_player_character (Utilities|Casting|CastToBP_DefaultPlayerCharacter (Game|Player|GetPlayerPawn 0)))
  (Variables|Default|SetPlayerCharacterRef _asbp_default_player_character)
  (Variables|Default|SetDilation (Class|GameplayStatics|GetGlobalTimeDilation))
  (Variables|Default|SetNormalPlayerTimeDilation (Class|Actor|GetActorTimeDilation (Variables|Default|GetPlayerCharacterRef))))

(event EventOnWildcardEnd
  (bind _playercharacterref (Variables|Default|GetPlayerCharacterRef))
  (bind _camcomp (Variables|/Script/SUL_COLLAB_2026.PlayerCharacter|GetCamComp _playercharacterref))
  (Audio|PlaySound2D "/Game/Blueprint/Shez/Za_Warudo_The_World_Time_Resume.Za_Warudo_The_World_Time_Resume" 1.0 1.0 0.0 0 0)
  ;[0.15 0.15 0.15 0.5] End Delay takes current time dialation into account (0.01% of standard, this delay will last 1.5 real seconds
  (Utilities|FlowControl|Delay 0.015)
  (bind _structout (Utilities|Struct|SetmembersinPostProcessSettings (Variables|/Script/Engine.CameraComponent|GetPostProcessSettings _camcomp) "(X=1.000000,Y=1.000000,Z=1.000000,W=1.000000)"))
  (Variables|/Script/Engine.CameraComponent|SetPostProcessSettings _camcomp _structout)
  (Development|PrintString "Undo effects of wildcard.")
  (Default|CallWildcardFinished)
  (Utilities|Time|SetGlobalTimeDilation (Variables|Default|GetDilation))
  (Variables|/Script/Engine.Actor|SetCustomTimeDilation (Variables|Default|GetPlayerCharacterRef) (Variables|Default|GetNormalPlayerTimeDilation))
  (Variables|/Game/Blueprint/DefaultBlueprint/BP_DefaultPlayerCharacter.BP_DefaultPlayerCharacter_C|SetWildcardActive? (Variables|Default|GetPlayerCharacterRef) false))

(event EventOnWildcardActivate
  (bind _playercharacterref (Variables|Default|GetPlayerCharacterRef))
  (bind _camcomp (Variables|/Script/SUL_COLLAB_2026.PlayerCharacter|GetCamComp _playercharacterref))
  (Audio|PlaySound2D "/Game/Blueprint/Shez/_Za_Warudo__Sound_Effect._Za_Warudo__Sound_Effect" 1.0 1.0 0.0 0 0)
  (Utilities|FlowControl|Delay 2.0)
  (Variables|Default|SetDefault%20Post%20Process (Variables|/Script/Engine.CameraComponent|GetPostProcessSettings _camcomp))
  (bind _structout (Utilities|Struct|SetmembersinPostProcessSettings (Variables|/Script/Engine.CameraComponent|GetPostProcessSettings _camcomp) (Variables|Default|GetSaturation) (Variables|Default|GetGain) (Variables|Default|GetOffset)))
  (Variables|/Script/Engine.CameraComponent|SetPostProcessSettings _camcomp _structout)
  (Class|BaseWildcard|RunWildcardTimer)
  ;[0.15 0.15 0.15 0.5] multiply time by 0.01  to get dialated delay in real seconds
  (Utilities|Time|SetGlobalTimeDilation 0.01)
  (Utilities|FlowControl|Delay 0.001)
  (Variables|/Script/Engine.Actor|SetCustomTimeDilation (Variables|Default|GetPlayerCharacterRef) 1e+02))

(fn ConstructionScript)