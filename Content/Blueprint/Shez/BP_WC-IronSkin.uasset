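; Iron Skin wildcard pickup that turns on damage mitigation for the player while active.
; Any overlap on its sphere stores it as the player character's wildcard, using a reference cached on BeginPlay.
; Activation plays a sound, sets the player's mitigation flag and starts the wildcard timer.
; The end event plays a sound, then after a short delay clears the mitigation and wildcard-active flags.
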(event OnComponentBeginOverlap(Sphere)
  (params (OverlappedComponent :type Primitive%20Component%20Object%20Reference) (OtherActor :type Actor%20Object%20Reference) (OtherComp :type Primitive%20Component%20Object%20Reference) (OtherBodyIndex :type Integer) (bFromSweep :type Boolean) (SweepResult :type Hit%20Result%20Structure%20%28by%20ref%29))
  (Variables|/Game/Blueprint/DefaultBlueprint/BP_DefaultPlayerCharacter.BP_DefaultPlayerCharacter_C|SetAs%20BP%20Wildcard%20Example (Variables|Default|GetPlayerCharacterRef) (Utilities|ResolveSoftReference self)))

(event EventBeginPlay
  (bind _asbp_default_player_character (Utilities|Casting|CastToBP_DefaultPlayerCharacter (Game|Player|GetPlayerPawn 0)))
  (Variables|Default|SetPlayerCharacterRef _asbp_default_player_character))

(event EventOnWildcardEnd
  (Audio|PlaySound2D "/Game/Blueprint/Shez/Za_Warudo_The_World_Time_Resume.Za_Warudo_The_World_Time_Resume" 1.0 1.0 0.0 0 0)
  (Utilities|FlowControl|Delay 1.5)
  (Variables|/Game/Blueprint/DefaultBlueprint/BP_DefaultPlayerCharacter.BP_DefaultPlayerCharacter_C|SetMitigationActive? (Variables|Default|GetPlayerCharacterRef) false)
  (Development|PrintString "Undo effects of wildcard.")
  (Variables|/Game/Blueprint/DefaultBlueprint/BP_DefaultPlayerCharacter.BP_DefaultPlayerCharacter_C|SetWildcardActive? (Variables|Default|GetPlayerCharacterRef) false))

(event EventOnWildcardActivate
  (Audio|PlaySound2D "/Engine/EngineSounds/1kSineTonePing.1kSineTonePing" 1.0 1.0 0.0 0 0)
  (Variables|/Game/Blueprint/DefaultBlueprint/BP_DefaultPlayerCharacter.BP_DefaultPlayerCharacter_C|SetMitigationActive? (Variables|Default|GetPlayerCharacterRef) true)
  (Class|BaseWildcard|RunWildcardTimer))

(fn ConstructionScript)