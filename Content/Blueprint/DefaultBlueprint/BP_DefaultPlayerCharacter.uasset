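; Default player character Blueprint that adds movement audio and camera feedback, and spawns an attached gun with a pickup event.
; Movement, slide and card-pickup dispatchers drive one-shot sounds, slide loops and motion blur for dashing and sliding.
; A reversible timeline shrinks the capsule and moves the camera during slides.
; Footsteps trigger by distance travelled, while a looping timer scales falling-wind volume by downward speed and landing picks hard or soft impacts.
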(event Custom|OnSlideStart_Event
  ;[0.15 0.15 0.15 0.5] Slide Transition
  (Audio|PlaySoundatLocation "/Game/Audio/PlayerMovement/Slide_Cue.Slide_Cue" (Transformation|GetActorLocation) "0, 0, 0" 1.0 1.0 0.0 0 0 0 0)
  (bind (_direction _slide _camera_height) (Timeline|SlideTimeline Play)
    (:Update
      (Components|Capsule|SetCapsuleHalfHeight (Variables|Default|GetCapsuleComponent) (* _slide (Variables|Default|GetDefault%20Height)) true)
      (Transformation|SetRelativeLocation (Variables|Default|GetCamComp) (Math|Vector|MakeVector 2e+01 0.0 _camera_height) false false))))

(event Custom|OnSlideEnd_Event
  (bind _slidesfx (Variables|Default|GetSlideSFX))
  ;[0.15 0.15 0.15 0.5] Slide Transition
  (Utilities|IsValid _slidesfx
    (:Is%20Valid
      (Audio|Components|Audio|Stop _slidesfx))
    (:Is%20Not%20Valid
      _))
  (CallFunction|ResetMotionBlur)
  (bind (_direction _slide _camera_height) (Timeline|SlideTimeline Reverse)
    (:Update
      (Components|Capsule|SetCapsuleHalfHeight (Variables|Default|GetCapsuleComponent) (* _slide (Variables|Default|GetDefault%20Height)) true)
      (Transformation|SetRelativeLocation (Variables|Default|GetCamComp) (Math|Vector|MakeVector 2e+01 0.0 _camera_height) false false))))

(event Custom|Reset%20Dash%20FX
  (CallFunction|ResetMotionBlur))

(event Custom|Turn%20Of%20Loop%20SFX
  (bind _slidesfx (Variables|Default|GetSlideSFX))
  (bind _fallingsfx (Variables|Default|GetFallingSFX))
  (Utilities|IsValid _slidesfx
    (:Is%20Valid
      (Audio|Components|Audio|Stop _slidesfx)
      (Utilities|IsValid _fallingsfx
        (:Is%20Valid
          (Audio|Components|Audio|Stop _fallingsfx))))))

(event Custom|PlayJumpSFX
  (if (AI|Components|NavMovement|IsMovingonGround (Variables|Character|GetCharacterMovement))
    (Audio|PlaySoundatLocation "/Game/Audio/PlayerMovement/Jump_Cue.Jump_Cue" (Transformation|GetActorLocation) "0, 0, 0" 1.0 1.0 0.0 0 0 0 0)))

(event Custom|PlayDash%20FX
  (Audio|PlaySoundatLocation "/Game/Audio/PlayerMovement/Dash_Cue.Dash_Cue" (Transformation|GetActorLocation) "0, 0, 0" 1.0 1.0 0.0 0 0 0 0)
  (Variables|/Script/Engine.CameraComponent|SetPostProcessSettings (Variables|Default|GetCamComp) (Utilities|Struct|MakePostProcessSettings 2.5 7.5)))

(event Custom|Walking%20Step
  (bind _charactermovement (Variables|Character|GetCharacterMovement))
  (bind _velocity (Variables|/Script/Engine.MovementComponent|GetVelocity _charactermovement))
  ;[0.15 0.15 0.15 0.5] Check if player can make steping sound
  (if (AI|Components|NavMovement|IsMovingonGround (Variables|Character|GetCharacterMovement))
    (if (Variables|Default|GetCan%20Step)
      (Audio|PlaySoundatLocation "/Game/Audio/PlayerMovement/FootStep.FootStep" (Transformation|GetActorLocation) "0, 0, 0" 1.0 1.0 0.0 0 0 0 0)
      (Variables|Default|SetCan%20Step false)
      (else
        ;[0.15 0.15 0.15 0.5] Update distance traveled
        (bind _output_get (Variables|Default|SetDistanceTravel (+ (* (Math|Vector2D|Vector2DLength (Math|Vector2D|MakeVector2D (.x _velocity) (.y _velocity))) (Utilities|Time|GetWorldDeltaSeconds)) (Variables|Default|GetDistanceTravel))))
        (if (>= _output_get (Variables|Default|GetDistancePerStep))
          (CallFunction|ResetStep))))
    (else
      (CallFunction|ResetStep))))

(event Custom|Reset%20Step
  ;[0.15 0.15 0.15 0.5] Reset travel and step
  (Variables|Default|SetDistanceTravel 0.0)
  (Variables|Default|SetCan%20Step true))

(event Custom|Start%20Slide%20Sound
  ;[0.15 0.15 0.15 0.5] Play Sound when start sliding on surface
  (bind _returnvalue (Audio|SpawnSoundAttached "/Game/Audio/PlayerMovement/SlideLoop.SlideLoop" (Variables|Default|GetCapsuleComponent) "None" "0, 0, 0" "0, 0, 0" "KeepRelativeOffset" false 1.0 1.0 0.0 0 0))
  (Variables|Default|SetSlideSFX _returnvalue)
  (Variables|/Script/Engine.CameraComponent|SetPostProcessSettings (Variables|Default|GetCamComp) (Utilities|Struct|MakePostProcessSettings 1.0)))

(event Custom|End%20Slide%20Sound
  (bind _slidesfx (Variables|Default|GetSlideSFX))
  ;[0.15 0.15 0.15 0.5] Stop Playing sound on Not slide on surface
  (Utilities|IsValid _slidesfx
    (:Is%20Valid
      (Audio|Components|Audio|Stop _slidesfx)
      (CallFunction|ResetMotionBlur))))

(event Custom|CustomEvent
  (Audio|PlaySound2D "/Game/Audio/Wildcard/card_draw_3_Cue.card_draw_3_Cue" 1.0 1.0 0.0 0 0))

(event Custom|Check%20Fall%20Speed
  ;[0.15 0.15 0.15 0.5] When player is falling
  (if (>= (CallFunction|GetDownSpeed) (Variables|Default|GetMinFallSpeed))
    (if (Variables|Default|GetFallingDown)
      (Utilities|IsValid (Variables|Default|GetFallingSFX)
        (:Is%20Valid
          (Audio|Components|Audio|SetVolumeMultiplier (Variables|Default|GetFallingSFX) (/ (- (CallFunction|GetDownSpeed) (Variables|Default|GetMinFallSpeed)) (Variables|Default|GetRangeOfFallSpeed)) :!class /Script/Engine.AudioComponent)))
      (else
        (bind _returnvalue (Audio|SpawnSoundAttached "/Game/Audio/PlayerMovement/Player_Falling_Loop__Cue.Player_Falling_Loop__Cue" (Variables|Default|GetCapsuleComponent) "None" "0, 0, 0" "0, 0, 0" "KeepRelativeOffset" false 1.0 1.0 0.0 0 0))
        (Variables|Default|SetFallingSFX _returnvalue)
        (Variables|Default|SetFallingDown true)))
    (elif (Variables|Default|GetFallingDown)
      (Utilities|IsValid (Variables|Default|GetFallingSFX)
        (:Is%20Valid
          (Audio|Components|Audio|Stop (Variables|Default|GetFallingSFX)))))))

(event EventPickUpGun
  (Variables|Default|SetHasGun true)
  (Audio|PlaySoundatLocation "/Game/Audio/Gun/PickUp_Cue.PickUp_Cue" (Transformation|GetWorldLocation (Variables|Default|GetGunPos)) "0, 0, 0" 1.0 1.0 0.0 0 0 0 0)
  (Rendering|SetActorHiddenInGame (Variables|Default|GetGun) false))

(event Game|Damage|EventAnyDamage
  (params (Damage :type Float%20%28single-precision%29) (DamageType :type Damage%20Type%20Object%20Reference) (InstigatedBy :type Controller%20Object%20Reference) (DamageCauser :type Actor%20Object%20Reference))
  (if (not (<= (- (Math|Float|Truncate Damage) (Variables|/Script/SUL_COLLAB_2026.HealthComponent|GetCurrentHealth (Variables|Default|GetHealthComp))) 0))
    (CallFunction|TurnOfLoopSFX)))

(event EventOnLanded
  (params (Hit :type Hit%20Result%20Structure%20%28by%20ref%29))
  (bind _returnvalue (Transformation|GetActorLocation))
  (bind _fallingsfx (Variables|Default|GetFallingSFX))
  ;[0.15 0.15 0.15 0.5] Player landed#
  (Utilities|IsValid _fallingsfx
    (:Is%20Valid
      (Audio|Components|Audio|Stop _fallingsfx)
      (Utilities|Time|PauseTimerbyHandle (Variables|Default|GetFallingTImer))
      (if (>= (CallFunction|GetDownSpeed) (Variables|Default|GetMaxFallSoundSpeed))
        (Audio|PlaySoundatLocation "/Game/Audio/PlayerMovement/HardLanded.HardLanded" _returnvalue "0, 0, 0" 1.0 1.0 0.0 0 0 0 0)
        (else
          (Audio|PlaySoundatLocation "/Game/Audio/PlayerMovement/SoftLanding.SoftLanding" _returnvalue "0, 0, 0" 1.0 1.0 0.0 0 0 0 0))))))

(event EventOnMovementModeChanged
  (params (PrevMovementMode :type EMovementMode%20Enum :default "MOVE_None") (NewMovementMode :type EMovementMode%20Enum :default "MOVE_None") (PrevCustomMode :type Byte :default 0) (NewCustomMode :type Byte :default 0))
  ;[0.15 0.15 0.15 0.5] When player is falling
  (if (Utilities|Enum|Equal(Enum) NewMovementMode "MOVE_Falling")
    (bind _returnvalue (Utilities|Time|SetTimerbyEvent (delegate Custom|Check%20Fall%20Speed) (Utilities|Time|GetWorldDeltaSeconds) true))
    (Variables|Default|SetFallingTImer _returnvalue)
    (Variables|Default|SetFallingDown false)))

(event EventBeginPlay
  (bind _gunpos (Variables|Default|GetGunPos))
  (Utilities|FlowControl|Sequence
    (:then_0
      ;[0.15 0.15 0.15 0.5] Set Gun
      (bind _returnvalue (Game|SpawnActorfromClass "/Game/Blueprint/DefaultBlueprint/BP_Gun.BP_Gun_C" (Math|Transform|MakeTransform (Variables|/Script/Engine.SceneComponent|GetRelativeLocation _gunpos) (Variables|/Script/Engine.SceneComponent|GetRelativeRotation _gunpos) "1.000000,1.000000,1.000000") "Undefined" "MultiplyWithRoot" 0 0))
      (bind _output_get (Variables|Default|SetGun _returnvalue))
      (Transformation|AttachComponentToComponent _output_get (Variables|Default|GetCamComp) "None" "KeepRelative" "KeepRelative" "KeepRelative" true)
      (Variables|Default|SetRangeOfFallSpeed (- (Variables|Default|GetMaxFallSoundSpeed) (Variables|Default|GetMinFallSpeed))))
    (:then_1
      (Variables|Default|SetDefault%20Height (Components|Capsule|GetUnscaledCapsuleHalfHeight (Variables|Default|GetCapsuleComponent))))
    (:then_2
      (EventDispatchers|BindEventtoOnSlideStart (delegate Custom|OnSlideStart_Event))
      (EventDispatchers|AssignOnSlideEnd (delegate Custom|OnSlideEnd_Event))
      (EventDispatchers|BindEventtoOnJump (delegate Custom|PlayJumpSFX))
      (EventDispatchers|BindEventtoOnDash (delegate Custom|PlayDash%20FX))
      (EventDispatchers|BindEventtoOnStopDash (delegate Custom|Reset%20Dash%20FX))
      (EventDispatchers|AssignOnWalking (delegate Custom|Walking%20Step))
      (EventDispatchers|BindEventtoStopWalking (EventDispatchers|CreateEvent :!event Custom|Reset%20Step))
      (EventDispatchers|BindEventtoIsSliding (delegate Custom|Start%20Slide%20Sound))
      (EventDispatchers|BindEventtoIsNotSliding (delegate Custom|End%20Slide%20Sound))
      (EventDispatchers|BindEventtoPickUpCard (delegate Custom|CustomEvent)))))

(fn ConstructionScript)

(fn GetDownSpeed
  (return (* (.z (Variables|/Script/Engine.MovementComponent|GetVelocity (Variables|Character|GetCharacterMovement))) -1.0)))

(fn ResetMotionBlur
  (Variables|/Script/Engine.CameraComponent|SetPostProcessSettings (Variables|Default|GetCamComp) (Utilities|Struct|MakePostProcessSettings 0.0 0.0)))