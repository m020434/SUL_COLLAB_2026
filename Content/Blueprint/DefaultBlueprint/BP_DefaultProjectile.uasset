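; Default projectile Blueprint that reports its impact and destroys itself when it hits something.
; The construction script copies Speed and Gravity into the projectile movement component, so initial and max speed are equal.
; On hit, it passes the other actor and hit result to CallProjectileImpact, then spawns the player projectile impact effect at the hit location.
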(event EventOnHit
  (params (OtherActor :type Actor%20Object%20Reference) (HitResult :type Hit%20Result%20Structure))
  (Default|CallProjectileImpact OtherActor HitResult)
  (Niagara|SpawnSystematLocation "/Game/Juno/VFX/N_PlayerProjectile_Impact.N_PlayerProjectile_Impact" (.Location (Collision|BreakHitResult HitResult)))
  (Actor|DestroyActor))

(fn ConstructionScript
  (bind _projectilemovementcomp (Variables|Default|GetProjectileMovementComp))
  (Variables|/Script/Engine.ProjectileMovementComponent|SetInitialSpeed _projectilemovementcomp (Variables|Default|Getspeed))
  (Variables|/Script/Engine.ProjectileMovementComponent|SetMaxSpeed _projectilemovementcomp (Variables|Default|Getspeed))
  (Variables|/Script/Engine.ProjectileMovementComponent|SetProjectileGravityScale _projectilemovementcomp (Variables|Default|Getgravity)))