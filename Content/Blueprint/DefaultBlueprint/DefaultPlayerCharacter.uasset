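; Default player character Blueprint that handles slide audio, capsule height changes for sliding, and a debug popup.
; The R debug key adds a reactive popup widget, spawns an attached slide sound and binds its playback to slide start and stop dispatchers.
; Height events play or reverse a timeline that sets capsule half height, though its Slide value is multiplied by zero.
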(event Custom|Slide%20noise
  (Audio|Components|Audio|Play (Variables|Default|GetSlide%20sound) 0.0))

(event Custom|OnStopSliding_Event
  (Audio|Components|Audio|Stop (Variables|Default|GetSlide%20sound)))

(event EventBeginPlay)

(event Collision|EventActorBeginOverlap
  (params (OtherActor :type Actor%20Object%20Reference)))

(event EventTick
  (params (DeltaSeconds :type Float%20%28single-precision%29)))

(event EventChangetoDefaultHeight
  (bind _slide (Timeline|Timeline Reverse)
    (:Update
      (Components|Capsule|SetCapsuleHalfHeight (Variables|Default|GetCapsuleComponent) (* _slide 0.0) true))))

(event EventChangetoSlideHeight
  (bind _slide (Timeline|Timeline Play)
    (:Update
      (Components|Capsule|SetCapsuleHalfHeight (Variables|Default|GetCapsuleComponent) (* _slide 0.0) true))))

(event Input|KeyboardEvents|DebugKeyR
  (params (Key :type Key%20Structure :default "None") (ActionValue :type Input%20Action%20Value%20Structure))
  (:Pressed
    (bind _returnvalue (UserInterface|CreateWidget "/Game/Blueprint/Shez/UI/ReactiveMascot/WBP_ReactivePopupCore.WBP_ReactivePopupCore_C"))
    (UserInterface|Viewport|AddtoViewport _returnvalue 0)
    (bind _returnvalue_2 (Audio|SpawnSoundAttached "/Game/Audio/PlayerMovement/Slide_Cue.Slide_Cue" (Variables|Default|GetCapsuleComponent) "None" "0, 0, 0" "0, 0, 0" "KeepRelativeOffset" false 1.0 1.0 0.0 0 0))
    (Variables|Default|SetSlide%20sound _returnvalue_2)
    (EventDispatchers|BindEventtoOnSlideStart (delegate Custom|Slide%20noise))
    (EventDispatchers|AssignOnStopSliding (delegate Custom|OnStopSliding_Event))))

(fn ConstructionScript)