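; Gun Blueprint that provides simple procedural shooting and reload animations, with no firing or reload logic in its graphs.
; ShootingAnimation and ReloadAnimation each restart their own Timeline, whose Pitch track drives the relative rotation of MeshComp in place of skeletal animation.
; The reload resets the mesh rotation to zero when it finishes, while the shooting animation is marked temporary and has no explicit reset.
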(event EventBeginPlay)

(event Collision|EventActorBeginOverlap
  (params (OtherActor :type Actor%20Object%20Reference)))

(event EventTick
  (params (DeltaSeconds :type Float%20%28single-precision%29)))

(event EventReloadAnimation
  ;[0.15 0.15 0.15 0.5] Temperary
  (bind _pitch (Timeline|Timeline_0 PlayFromStart)
    (:Update
      (Transformation|SetRelativeRotation (Variables|Default|GetMeshComp) (Math|Rotator|MakeRotator 0.0 _pitch 0.0) false false))
    (:Finished
      (Transformation|SetRelativeRotation (Variables|Default|GetMeshComp) (Math|Rotator|MakeRotator 0.0 0.0 0.0) false false))))

(event EventShootingAnimation
  ;[0.15 0.15 0.15 0.5] Temperary
  (bind _pitch (Timeline|Timeline PlayFromStart)
    (:Update
      (Transformation|SetRelativeRotation (Variables|Default|GetMeshComp) (Math|Rotator|MakeRotator 0.0 _pitch 0.0) false false))))

(fn ConstructionScript)