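; BP_Lava is a lava hazard that deals damage over time to the player, built on a parent class.
; Its AffectPlayer event starts a looping half-second timer that calls LavaDamage to apply fixed damage to PlayerCharacter.
; When an actor implementing BPI_Character leaves OverlapBox, the timer is cleared to stop the damage.
; Debug prints mark the hit, each damage tick and the stop.
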(event OnComponentEndOverlap(OverlapBox)
  (params (OverlappedComponent :type Primitive%20Component%20Object%20Reference) (OtherActor :type Actor%20Object%20Reference) (OtherComp :type Primitive%20Component%20Object%20Reference) (OtherBodyIndex :type Integer))
  (if (Utilities|DoesObjectImplementInterface OtherActor "/Game/Blueprint/Damian/DEV_Blueprints/Objects/BPI_Character.BPI_Character_C")
    (Utilities|Time|ClearandInvalidateTimerbyHandle (Variables|Default|GetLava%20Timer))
    (Development|PrintString "stop damage")))

(event Custom|LavaDamage
  (Game|Damage|ApplyDamage (stale EventAffectPlayer Player%20Character) 1e+01 0 0)
  (Development|PrintString "damage"))

(event EventBeginPlay
  (|CallParentFunction) ; This node is disabled and will not be called.\nDrag off pins to build functionality.
)

(event EventTick
  (params (DeltaSeconds :type Float%20%28single-precision%29))
  (|CallParentFunction DeltaSeconds) ; This node is disabled and will not be called.\nDrag off pins to build functionality.
)

(event EventAffectPlayer
  (params (Player%20Character :type BP%20Default%20Player%20Character%20Object%20Reference))
  (bind _returnvalue (Utilities|Time|SetTimerbyEvent (delegate Custom|LavaDamage) 0.5 true))
  (Variables|Default|SetLava%20Timer _returnvalue)
  (Development|PrintString "hit"))

(event EventActorBeginOverlap
  (params (OtherActor :type Actor%20Object%20Reference))
  (|CallParentFunction OtherActor))

(fn ConstructionScript
  (|CallParentFunction))