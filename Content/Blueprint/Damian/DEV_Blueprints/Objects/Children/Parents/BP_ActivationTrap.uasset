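; BP_ActivationTrap is a spike trap that moves its Spike component shortly after AffectPlayer triggers it.
; BeginPlay stores the spike's world location, and AffectPlayer starts a short timer if the trap is not already active.
; The timer plays a timeline that lerps the spike toward the start location plus an EndLocation offset.
; An Activated flag blocks retriggering until the timeline finishes.
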(event Custom|Initialise
  (Variables|Default|SetStartLocation (Transformation|GetWorldLocation (Variables|Default|GetSpike))))

(event Custom|Spikes
  (bind _startlocation (Variables|Default|GetStartLocation))
  (bind _looping_movement (Timeline|Timeline PlayFromStart)
    (:Update
      (Transformation|SetWorldLocation (Variables|Default|GetSpike) (Math|Vector|Lerp(Vector) _startlocation (+ _startlocation (Variables|Default|GetEndLocation)) _looping_movement) false false))
    (:Finished
      (Variables|Default|SetActivated false))))

(event Collision|EventActorBeginOverlap
  (params (OtherActor :type Actor%20Object%20Reference))
  (|CallParentFunction OtherActor) ; This node is disabled and will not be called.\nDrag off pins to build functionality.
)

(event EventTick
  (params (DeltaSeconds :type Float%20%28single-precision%29))
  (|CallParentFunction DeltaSeconds) ; This node is disabled and will not be called.\nDrag off pins to build functionality.
)

(event EventAffectPlayer
  (params (Player%20Character :type BP%20Default%20Player%20Character%20Object%20Reference))
  (if (not (Variables|Default|GetActivated))
    (Variables|Default|SetActivated true)
    (Utilities|Time|SetTimerbyEvent (delegate Custom|Spikes) 0.25)))

(event EventBeginPlay
  (CallFunction|Initialise))

(fn ConstructionScript
  (|CallParentFunction))