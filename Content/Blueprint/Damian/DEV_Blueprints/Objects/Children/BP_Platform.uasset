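; BP_Platform is a child object Blueprint for a platform that moves after its AffectPlayer event fires, likely a falling platform given the "Falls" track.
; A guarded one-second timer disables the overlap box and plays a timeline that lerps the actor from its BeginPlay location by an EndLocation offset.
; When the timeline finishes, it restores collision on the box and clears the guard for retriggering, with debug prints left in.
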(event Custom|Initialise
  (Variables|Default|SetStart%20Location (Transformation|GetActorLocation)))

(event Custom|Activate%20Platform
  (bind _start_location (Variables|Default|GetStart%20Location))
  (Collision|SetCollisionEnabled (Variables|Default|GetOverlap%20Box) "NoCollision")
  (bind _falls (Timeline|Timeline PlayFromStart)
    (:Update
      (Transformation|SetActorLocation (Math|Vector|Lerp(Vector) _start_location (+ _start_location (Variables|Default|GetEnd%20Location)) _falls) false false)
      (Development|PrintString "Platform Moved"))
    (:Finished
      (Variables|Default|SetActivated false)
      (Collision|SetCollisionEnabled (Variables|Default|GetOverlap%20Box) "QueryAndPhysics")
      (Development|PrintString "No platform collision"))))

(event Collision|EventActorBeginOverlap
  (params (OtherActor :type Actor%20Object%20Reference))
  (|CallParentFunction OtherActor) ; This node is disabled and will not be called.\nDrag off pins to build functionality.
)

(event EventTick
  (params (DeltaSeconds :type Float%20%28single-precision%29))
  (|CallParentFunction DeltaSeconds) ; This node is disabled and will not be called.\nDrag off pins to build functionality.
)

(event EventAffectPlayer
  (params (Player%20Character :type BP%20Default%20Player%20Character%20Object%20Reference))
  (if (not (Variables|Default|GetActivated))
    (Variables|Default|SetActivated true)
    (Utilities|Time|SetTimerbyEvent (delegate Custom|Activate%20Platform) 1.0)))

(event EventBeginPlay
  (CallFunction|Initialise))

(fn ConstructionScript
  (|CallParentFunction))