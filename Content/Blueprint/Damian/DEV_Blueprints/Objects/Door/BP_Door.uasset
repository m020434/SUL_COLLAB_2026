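; BP_Door is a door that slides open once when its OpenDoor event is triggered.
; BeginPlay caches the actor's location, and OpenDoor, which also calls the parent version, plays a Timeline behind a DoOnce.
; The Timeline lerps the Cube's world location from that start to start plus EndLocation, used as an offset, and prints a debug "Hello" on every update.
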(event Collision|EventActorBeginOverlap
  (params (OtherActor :type Actor%20Object%20Reference))
  (|CallParentFunction OtherActor) ; This node is disabled and will not be called.\nDrag off pins to build functionality.
)

(event EventTick
  (params (DeltaSeconds :type Float%20%28single-precision%29))
  (|CallParentFunction DeltaSeconds) ; This node is disabled and will not be called.\nDrag off pins to build functionality.
)

(event EventOpenDoor
  (bind _start_location (Variables|Default|GetStart%20Location))
  (|CallParentFunction)
  (Utilities|FlowControl|DoOnce false
    (:Completed
      (bind _open_door (Timeline|Timeline Play)
        (:Update
          (Transformation|SetWorldLocation (Variables|Default|GetCube) (Math|Vector|Lerp(Vector) _start_location (+ _start_location (Variables|Default|GetEnd%20Location)) _open_door) false false)
          (Development|PrintString "Hello"))))))

(event EventBeginPlay
  (|CallParentFunction)
  (Variables|Default|SetStart%20Location (Transformation|GetActorLocation)))

(fn ConstructionScript
  (|CallParentFunction))