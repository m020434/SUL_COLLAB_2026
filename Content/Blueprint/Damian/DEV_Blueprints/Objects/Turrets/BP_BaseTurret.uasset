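; BP_BaseTurret is a base turret that fires Dev_BP_Projectile while a character is inside its detection area.
; Detection overlap with a BPI_Character actor starts a looping timer that spawns projectiles at the Arrow component's transform every ShootSpeed seconds, and leaving clears it.
; Incoming damage lowers a clamped CurrentHealth, but only prints a debug string while health remains, with no death handling.
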(event OnComponentBeginOverlap(Detection)
  (params (OverlappedComponent :type Primitive%20Component%20Object%20Reference) (OtherActor :type Actor%20Object%20Reference) (OtherComp :type Primitive%20Component%20Object%20Reference) (OtherBodyIndex :type Integer) (bFromSweep :type Boolean) (SweepResult :type Hit%20Result%20Structure%20%28by%20ref%29))
  (if (Utilities|DoesObjectImplementInterface OtherActor "/Game/Blueprint/Damian/DEV_Blueprints/Objects/BPI_Character.BPI_Character_C")
    (CallFunction|StartShootingTimer)
    (Development|PrintString "Hello")))

(event OnComponentEndOverlap(Detection)
  (params (OverlappedComponent :type Primitive%20Component%20Object%20Reference) (OtherActor :type Actor%20Object%20Reference) (OtherComp :type Primitive%20Component%20Object%20Reference) (OtherBodyIndex :type Integer))
  (if (Utilities|DoesObjectImplementInterface OtherActor "/Game/Blueprint/Damian/DEV_Blueprints/Objects/BPI_Character.BPI_Character_C")
    (Utilities|Time|ClearandInvalidateTimerbyHandle (Variables|Default|GetShootTimer))))

(event Custom|StartShootingTimer
  (bind _returnvalue (Utilities|Time|SetTimerbyEvent (delegate Custom|Shoot) (Variables|Default|GetShootSpeed) true))
  (Variables|Default|SetShootTimer _returnvalue)
  (Development|PrintString "start"))

(event Custom|Shoot
  (bind _arrow (Variables|Default|GetArrow))
  (Game|SpawnActorfromClass "/Game/Blueprint/Damian/DEV_Blueprints/Traps/Dev_BP_Projectile.Dev_BP_Projectile_C" (Math|Transform|MakeTransform (Transformation|GetWorldLocation _arrow) (Transformation|GetWorldRotation _arrow) "1.000000,1.000000,1.000000") "Undefined" "MultiplyWithRoot" 0 0)
  (Development|PrintString "shoot"))

(event Game|Damage|EventAnyDamage
  (params (Damage :type Float%20%28single-precision%29) (DamageType :type Damage%20Type%20Object%20Reference) (InstigatedBy :type Controller%20Object%20Reference) (DamageCauser :type Actor%20Object%20Reference))
  ;[0.15 0.15 0.15 0.5] Health?
  (Variables|Default|SetCurrentHealth (Math|Float|Clamp(Float) (- (Variables|Default|GetCurrentHealth) Damage) 0.0 1e+02))
  (if (not (<= (Variables|Default|GetCurrentHealth) 0.0))
    (Development|PrintString "Hello")))

(fn ConstructionScript)