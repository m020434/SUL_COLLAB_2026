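; Turret actor that tracks the first player's character and fires projectiles at it.
; Every tick it snaps the Head component's world rotation to look at the player's location.
; A Shoot event, not triggered within this graph, spawns a Dev_BP_Projectile at the Arrow component, oriented toward the player's position at that moment.
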(event Custom|Aim%20At%20Player
  (bind _returnvalue (Game|GetPlayerCharacter 0))
  (bind _head (Variables|Default|GetHead))
  (Utilities|IsValid _returnvalue
    (:Is%20Valid
      (Transformation|SetWorldRotation _head (Math|Rotator|FindLookatRotation (Transformation|GetWorldLocation _head) (Transformation|GetActorLocation _returnvalue)) false false))))

(event EventBeginPlay
  (|CallParentFunction) ; This node is disabled and will not be called.\nDrag off pins to build functionality.
)

(event Collision|EventActorBeginOverlap
  (params (OtherActor :type Actor%20Object%20Reference))
  (|CallParentFunction OtherActor) ; This node is disabled and will not be called.\nDrag off pins to build functionality.
)

(event EventShoot
  (bind _returnvalue (Game|GetPlayerCharacter 0))
  (bind _arrow (Variables|Default|GetArrow))
  (bind _returnvalue_2 (Transformation|GetWorldLocation _arrow))
  (Utilities|IsValid _returnvalue
    (:Is%20Valid
      (Game|SpawnActorfromClass "/Game/Blueprint/Damian/DEV_Blueprints/Traps/Dev_BP_Projectile.Dev_BP_Projectile_C" (Math|Transform|MakeTransform _returnvalue_2 (Math|Rotator|FindLookatRotation _returnvalue_2 (Transformation|GetActorLocation _returnvalue)) "1.000000,1.000000,1.000000") "Undefined" "MultiplyWithRoot" 0 0))))

(event EventTick
  (params (DeltaSeconds :type Float%20%28single-precision%29))
  (CallFunction|AimatPlayer))

(fn ConstructionScript
  (|CallParentFunction))