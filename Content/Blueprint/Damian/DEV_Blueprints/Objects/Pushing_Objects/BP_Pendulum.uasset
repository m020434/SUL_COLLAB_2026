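; BP_Pendulum is a swinging pendulum obstacle whose Cube rotates on a timeline.
; InitialisePlatform stores the actor's rotation, but nothing in this Blueprint calls it.
; On BeginPlay, the MovingTrap timeline drives the Cube's relative rotation, lerping between that stored rotation and its negation via the LoopingMovement track.
; The Cube's overlap event is empty, and the damage and rotation-reset nodes are disconnected.
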(event OnComponentBeginOverlap(Cube)
  (params (OverlappedComponent :type Primitive%20Component%20Object%20Reference) (OtherActor :type Actor%20Object%20Reference) (OtherComp :type Primitive%20Component%20Object%20Reference) (OtherBodyIndex :type Integer) (bFromSweep :type Boolean) (SweepResult :type Hit%20Result%20Structure%20%28by%20ref%29)))

(event Custom|Initialise%20Platform
  (Variables|Default|SetRotation (Transformation|GetActorRotation)))

(event EventBeginPlay
  (bind _rotation (Variables|Default|GetRotation))
  (bind _looping_movement (Timeline|Moving%20Trap Play)
    (:Update
      (Transformation|SetRelativeRotation (Variables|Default|GetCube) (Math|Rotator|Lerp(Rotator) _rotation (* _rotation -1.0) _looping_movement) false false))))

(fn ConstructionScript)