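; BP_FanToLand is a fan obstacle that pushes the player character along its Arrow's forward direction.
; A Box trigger, sized at BeginPlay from AreaImpulse and LineExtend, starts a fast looping timer when the player enters.
; Each tick of that timer sphere-traces for Pawns along the arrow, with debug drawing, and launches the player on a hit.
; End overlap does nothing, as the timer-clearing logic is disconnected, so the timer keeps running.
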(event OnComponentBeginOverlap(Box)
  (params (OverlappedComponent :type Primitive%20Component%20Object%20Reference) (OtherActor :type Actor%20Object%20Reference) (OtherComp :type Primitive%20Component%20Object%20Reference) (OtherBodyIndex :type Integer) (bFromSweep :type Boolean) (SweepResult :type Hit%20Result%20Structure%20%28by%20ref%29))
  (if (== OtherActor (Game|GetPlayerCharacter 0))
    (bind _returnvalue (Utilities|Time|SetTimerbyEvent (delegate Custom|Wind%20Push) 0.03 true))))

(event OnComponentEndOverlap(Box)
  (params (OverlappedComponent :type Primitive%20Component%20Object%20Reference) (OtherActor :type Actor%20Object%20Reference) (OtherComp :type Primitive%20Component%20Object%20Reference) (OtherBodyIndex :type Integer)))

(event Custom|Wind%20Push
  (bind _returnvalue (Game|GetPlayerCharacter 0))
  (bind _arrow (Variables|Default|GetArrow))
  (bind _returnvalue_2 (Transformation|GetWorldLocation _arrow))
  (bind (_outhit _returnvalue_3) (Collision|SphereTraceForObjects _returnvalue_2 (+ _returnvalue_2 (* (Math|Vector|GetForwardVector _arrow) (Variables|Default|GetLine%20Extend))) (Variables|Default|GetAreaImpulse) (Utilities|Array|MakeArray "ObjectTypeQuery3") false 0 "ForDuration"))
  (if (and _returnvalue_3 (== (.HitActor (Collision|BreakHitResult _outhit)) _returnvalue))
    (Character|LaunchCharacter _returnvalue (* (Math|Vector|GetForwardVector (Variables|Default|GetArrow)) (Variables|Default|GetImpulse%20Added)) false false)))

(event Collision|EventActorBeginOverlap
  (params (OtherActor :type Actor%20Object%20Reference)))

(event EventTick
  (params (DeltaSeconds :type Float%20%28single-precision%29)))

(event EventBeginPlay
  (bind _areaimpulse (Variables|Default|GetAreaImpulse))
  (bind _returnvalue (/ _areaimpulse 2.5))
  (Components|Box|SetBoxExtent (Variables|Default|GetBox) (Math|Vector|MakeVector _returnvalue (/ (Variables|Default|GetLine%20Extend) 3.0) _returnvalue) true))

(fn ConstructionScript)