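; BP_TimeTarget is a development target that works out score and time bonuses from how accurately it is hit.
; OnTargetHit stores the hit accuracy, then passes it to CalculateAccuracyBonus with a score curve and a time curve in turn.
; Both results are only printed as debug strings; this Blueprint does not apply them to score or timer.
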(event EventOnTargetHit
  (params (HitAccuracy :type Float%20%28single-precision%29))
  (Variables|Default|SetHit%20Accuracy HitAccuracy)
  (Utilities|FlowControl|Sequence
    (:then_0
      (bind _returnvalue (Class|BaseTarget|CalculateAccuracyBonus "/Game/Blueprint/Brandon/DevBlueprints/ScoreBonusCurve.ScoreBonusCurve" (Variables|Default|GetHit%20Accuracy))) ; For Score
      (Development|PrintString (Utilities|String|ToString(Text) (Utilities|Text|FormatText "Score Added: {scoreAdded}" _returnvalue))))
    (:then_1
      (bind _returnvalue_2 (Class|BaseTarget|CalculateAccuracyBonus "/Game/Blueprint/Brandon/DevBlueprints/TimeBonusCurve.TimeBonusCurve" (Variables|Default|GetHit%20Accuracy))) ; For Time
      (Development|PrintString (Utilities|String|ToString(Text) (Utilities|Text|FormatText "Time Added: {timeAdded}" _returnvalue_2))))))

(fn ConstructionScript)