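; BP_TestCardSpawner is a test spawner that keeps a card and its pickup available at its location.
; On BeginPlay a looping one-second timer checks whether the spawned card is still valid.
; When it is not, it spawns a new card and a pickup actor at its own transform and hands the card reference to the pickup.
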(event Custom|Spawn%20Card
  (bind _returnvalue (Transformation|GetActorTransform))
  (Utilities|IsValid (Variables|Default|GetSpawned%20Card)
    (:Is%20Not%20Valid
      (bind _returnvalue_2 (Game|SpawnActorfromClass (Variables|Default|GetSpawnCard) _returnvalue "Undefined" "MultiplyWithRoot" 0 0))
      (bind _output_get (Variables|Default|SetSpawned%20Card _returnvalue_2))
      (bind _returnvalue_3 (Game|SpawnActorfromClass (Variables|Default|GetSpawnPickUp) _returnvalue "Undefined" "MultiplyWithRoot" 0 0))
      (Default|AddCardReferace _returnvalue_3 _output_get))))

(event EventBeginPlay
  (Utilities|Time|SetTimerbyEvent (delegate Custom|Spawn%20Card) 1.0 true))

(event Collision|EventActorBeginOverlap
  (params (OtherActor :type Actor%20Object%20Reference)))

(event EventTick
  (params (DeltaSeconds :type Float%20%28single-precision%29)))

(fn ConstructionScript)